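; BP_MiniCamera is an actor that follows the player character horizontally from a fixed height, as its own Z never changes.
; BeginPlay casts player pawn 0 to BaseCharacter and caches it as PlayerCharacter.
; Every Tick it copies that character's X and Y into its own location without sweeping, leaving rotation untouched.
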(event `self.ReceiveBeginPlay`
  (bind _asbase_character (cast `BaseCharacter` (`GameplayStatics.GetPlayerPawn` 0)))
  (set `self.PlayerCharacter` _asbase_character))

(event `self.ReceiveTick`
  (params (DeltaSeconds :type "Float (single-precision)"))
  (`self.K2_SetActorLocation` (`KismetMathLibrary.MakeVector` (.x (`self.K2_GetActorLocation` (`self.PlayerCharacter`))) (.y (`self.K2_GetActorLocation` (`self.PlayerCharacter`))) (.z (`self.K2_GetActorLocation`)))))

(fn `UserConstructionScript`)